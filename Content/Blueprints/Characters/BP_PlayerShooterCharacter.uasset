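; Player shooter character Blueprint that adds a minimap to the HUD and handles its sprite on death.
; On BeginPlay it runs the parent logic, then creates a WBP_MiniMap widget for player controller 0 and adds it to the viewport.
; Every Tick it polls IsDead and, while true, calls DestroyComponent on its PaperSprite.
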(event EventBeginPlay
  (|CallParentFunction)
  (bind _returnvalue (UserInterface|CreateWidget "/Game/UI/WBP_MiniMap.WBP_MiniMap_C" (Game|GetPlayerController 0)))
  (UserInterface|Viewport|AddtoViewport _returnvalue 0))

(event Collision|EventActorBeginOverlap
  (params (OtherActor :type Actor%20Object%20Reference))
  (|CallParentFunction OtherActor) ; This node is disabled and will not be called.\nDrag off pins to build functionality.
)

(event EventTick
  (params (DeltaSeconds :type Float%20%28single-precision%29))
  (if (Class|ShooterCharacter|IsDead)
    (Components|DestroyComponent (Variables|Default|GetPaperSprite))))

(fn ConstructionScript
  (|CallParentFunction))